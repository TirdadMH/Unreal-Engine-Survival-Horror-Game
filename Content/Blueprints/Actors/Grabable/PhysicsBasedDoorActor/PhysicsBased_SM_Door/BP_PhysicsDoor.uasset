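; BP_PhysicsDoor is a grabbable door that the player swings open or closed by hand with camera-rotation input.
; Grabbing freezes player movement and look input and enables the door's input; releasing restores walking, look and disables it.
; While held, scaled horizontal input adds yaw directly to the Door component's relative rotation, unclamped.
; A dot product against the actor's forward vector flips the direction according to the player's side.
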(event `/Game/Blueprints/Interfaces/BPI_Grabable.GrabObject`
  (bind _returnvalue (`GameplayStatics.GetPlayerController` 0))
  ;[1 1 1] Grab Door
  (`CharacterMovementComponent.DisableMovement` (`Character.CharacterMovement` (`GameplayStatics.GetPlayerCharacter` 0)))
  (`Controller.SetIgnoreLookInput` _returnvalue true)
  (`self.EnableInput` _returnvalue))

(event `/Game/Blueprints/Interfaces/BPI_Grabable.ReleaseObject`
  (bind _returnvalue (`GameplayStatics.GetPlayerController` 0))
  ;[1 1 1] Release Door
  (`CharacterMovementComponent.SetMovementMode` (`Character.CharacterMovement` (`GameplayStatics.GetPlayerCharacter` 0)) "MOVE_Walking" 0)
  (`Controller.ResetIgnoreLookInput` _returnvalue)
  (`self.DisableInput` _returnvalue))

(event `EnhancedInput|/Game/EnhancedInputs/Camera/IA_CameraRotation`
  (params (ActionValue :type "Vector2D Structure") (ElapsedSeconds :type "Float (double-precision)") (TriggeredSeconds :type "Float (double-precision)") (InputAction :type "InputAction Object Reference" :default "/Game/EnhancedInputs/Camera/IA_CameraRotation.IA_CameraRotation"))
  ;[1 1 1] Grab Door
  (:`Triggered`
    (`self.MoveDoor` (* ActionValue_X 0.6))))

(event `MoveDoor`
  (params (Amount :type "Float (double-precision)"))
  (bind _door (`self.Door`))
  ;[1 1 1] Move Door
  (`SceneComponent.K2_SetRelativeRotation` _door (`KismetMathLibrary.ComposeRotators` (`SceneComponent.RelativeRotation` _door) (`KismetMathLibrary.MakeRotator` 0.0 0.0 (* Amount (`KismetMathLibrary.SelectFloat` -1.0 1.0 (>= (`KismetMathLibrary.Dot_VectorVector` (`KismetMathLibrary.Normal` (- (`self.K2_GetActorLocation` self) (`self.K2_GetActorLocation` (`GameplayStatics.GetPlayerCharacter` 0)))) (`self.GetActorForwardVector` self)) 0.0))))) false false))

(fn `UserConstructionScript`)