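; BP_HideActor is an interactable hiding spot, such as a locker, that moves the player in and out of hiding.
; Interact starts a looping per-frame timer that slides the player to the hide or exit point, then fires a finished-moving dispatcher and flips IsHiding.
; Collision, movement and inventory access are disabled while hidden.
; The AIC_Classic AI controller is notified on entry, to check whether it saw, and after exit.
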(event `self.ReceiveBeginPlay`
  ; Setting a player Ref and a Controller Ref for Player Character
  (bind _asl1_character (cast `/Game/GameBP/LevelOne/L1_Character` (`GameplayStatics.GetPlayerCharacter` 0)))
  (set `self.PlayerRef` _asl1_character)
  (bind _ashg_player_controller (cast `/Game/GameBP/HG_PlayerController` (`GameplayStatics.GetPlayerController` 0)))
  (set `self.ControllerRef` _ashg_player_controller))

(event `/Game/Blueprints/Interfaces/BPI_Intraction.Interact`
  (bind _playerref (`self.PlayerRef`))
  ; Interacting with actor
  (if (`/Game/GameBP/LevelOne/L1_Character.IsHiding` (`self.PlayerRef`))
    (bind _returnvalue (`KismetSystemLibrary.K2_SetTimerDelegate` (delegate `MoveCharacter`) (`GameplayStatics.GetWorldDeltaSeconds`) true))
    (else
      (`self.EnemySeeInteraction`)
      (`self.SetActorEnableCollision` _playerref false)
      (`CharacterMovementComponent.DisableMovement` (`Character.CharacterMovement` _playerref))
      (set `/Game/GameBP/HG_PlayerController.CanOpenInventory` false (`self.ControllerRef`))
      (bind _returnvalue_2 (`KismetSystemLibrary.K2_SetTimerDelegate` (delegate `MoveCharacter`) (`GameplayStatics.GetWorldDeltaSeconds`) true)))))

(event `MoveCharacter`
  (bind _playerref (`self.PlayerRef`))
  ; Interacting with actor
  (`self.K2_SetActorTransform` _playerref (`KismetMathLibrary.MakeTransform` (`KismetMathLibrary.VInterpTo_Constant` (`self.K2_GetActorLocation` _playerref) (`SceneComponent.K2_GetComponentLocation` (select `bool` (`/Game/GameBP/LevelOne/L1_Character.IsHiding` (`self.PlayerRef`)) :`false` (`self.HidingPosition`) :`true` (`self.ExitPosition`))) (`GameplayStatics.GetWorldDeltaSeconds`) 1000.0)) false false)
  (if (== (`self.K2_GetActorLocation` (`self.PlayerRef`)) (`SceneComponent.K2_GetComponentLocation` (select `bool` (`/Game/GameBP/LevelOne/L1_Character.IsHiding` (`self.PlayerRef`)) :`false` (`self.HidingPosition`) :`true` (`self.ExitPosition`) :!type "SceneComponent Object Reference")) :`ErrorTolerance` 0.01)
    (`KismetSystemLibrary.K2_ClearAndInvalidateTimerHandle` (stale `/Game/Blueprints/Interfaces/BPI_Intraction.Interact` _returnvalue_2))
    (`KismetSystemLibrary.K2_ClearAndInvalidateTimerHandle` (stale `/Game/Blueprints/Interfaces/BPI_Intraction.Interact` _returnvalue))
    (`self.FinishedMoving`)))

(event `FinishedMoving`
  (bind _playerref (`self.PlayerRef`))
  (bind _playerref_2 (`self.PlayerRef`))
  ; After Interactring with Actor
  (`self.FinishedMovingED`)
  (if (`/Game/GameBP/LevelOne/L1_Character.IsHiding` _playerref)
    (set `/Game/GameBP/LevelOne/L1_Character.IsHiding` false _playerref)
    (bind _asaic_classic (castclass `/Game/AI/Classic/AIC_Classic` "/Game/AI/Classic/AIC_Classic.AIC_Classic_C"))
    (bind _returnvalue (`GameplayStatics.GetActorOfClass` _asaic_classic))
    (message `/Game/Blueprints/Interfaces/BPI_PlayerHiding.LeftHidingSpot` _returnvalue)
    (`self.SetActorEnableCollision` _playerref_2 true)
    (`CharacterMovementComponent.SetMovementMode` (`Character.CharacterMovement` _playerref_2) "MOVE_Walking" 0)
    (set `/Game/GameBP/HG_PlayerController.CanOpenInventory` true (`self.ControllerRef`))
    (else
      (set `/Game/GameBP/LevelOne/L1_Character.IsHiding` true _playerref))))

(event `EnemySeeInteraction`
  ; Did enemy see player entering a hide actor? (eg. Locker)
  (bind _asaic_classic (castclass `/Game/AI/Classic/AIC_Classic` "/Game/AI/Classic/AIC_Classic.AIC_Classic_C"))
  (bind _returnvalue (`GameplayStatics.GetActorOfClass` _asaic_classic))
  (message `/Game/Blueprints/Interfaces/BPI_PlayerHiding.DidEnemySee` _returnvalue self))

(event `EnemyFoundPlayer`
  ; Did enemy see player entering a hide actor? (eg. Locker)
)

(fn `UserConstructionScript`)