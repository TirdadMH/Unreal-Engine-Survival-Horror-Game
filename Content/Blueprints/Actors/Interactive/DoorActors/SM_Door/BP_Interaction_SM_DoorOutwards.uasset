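; Interactive door actor that swings open to either side, based on where the player or AI opening it stands.
; A dot product against the door's forward vector picks the swing direction, and a timeline drives the mesh yaw, reversing to close.
; Player interaction toggles the door.
; AI_Classic entering the box opens or toggles it and blocks interaction until closing finishes, while leaving closes it.
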(event `self.Interact`
  (if (`self.CanInteract`)
    (`self.OpenDoor` (`self.PlayerRef`))))

(event `OpenDoor`
  (params (ActorRef :type "Pawn Object Reference"))
  ;[1 1 1] Door Interact
  (if (`self.IsDoorClosed`)
    (set `self.IsDoorClosed` false)
    (set `self.DotProduct` (`KismetMathLibrary.Dot_VectorVector` (`KismetMathLibrary.Normal` (- (`self.K2_GetActorLocation` self) (`self.K2_GetActorLocation` ActorRef))) (`self.GetActorForwardVector` self)))
    (bind (_direction _alpha) (`Timeline|OpenDoorTL` :!via `PlayFromStart` :!label _label)
      (:`Update`
        (`SceneComponent.K2_SetRelativeRotation` (`self.StaticMesh_1`) (`KismetMathLibrary.MakeRotator` 0.0 0.0 (`KismetMathLibrary.Lerp` 0.0 (`KismetMathLibrary.SelectFloat` 90.0 -90.0 (>= (`self.DotProduct`) 0.0)) _alpha)) false false))
      (:`Finished`
        (switch `ETimelineDirection` _direction
          (:`Backward`
            (set `self.CanInteract` true)))))
    (else
      (set `self.IsDoorClosed` true)
      (goto _label :!via `ReverseFromEnd`))))

(event `self.Box.OnComponentBeginOverlap`
  (params (OverlappedComponent :type "PrimitiveComponent Object Reference") (OtherActor :type "Actor Object Reference") (OtherComp :type "PrimitiveComponent Object Reference") (OtherBodyIndex :type Integer) (bFromSweep :type Boolean) (SweepResult :type "HitResult Structure (by ref)"))
  ;[1 1 1] Door Interact
  (bind _asai_classic (cast `/Game/AI/Classic/AI_Classic` OtherActor))
  (set `self.CanInteract` false)
  (`self.OpenDoor` _asai_classic))

(event `self.Box.OnComponentEndOverlap`
  (params (OverlappedComponent :type "PrimitiveComponent Object Reference") (OtherActor :type "Actor Object Reference") (OtherComp :type "PrimitiveComponent Object Reference") (OtherBodyIndex :type Integer))
  ;[1 1 1] Door Interact
  (cast `/Game/AI/Classic/AI_Classic` OtherActor)
  (if (not (`self.IsDoorClosed`))
    (set `self.IsDoorClosed` true)
    (goto _label :!via `ReverseFromEnd`)))

(fn `UserConstructionScript`
  (`parent.UserConstructionScript`))