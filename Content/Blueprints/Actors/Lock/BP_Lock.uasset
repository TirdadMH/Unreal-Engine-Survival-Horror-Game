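; Interactable four-dial combination lock that opens and removes itself and its dials when the code matches.
; BeginPlay spawns BP_LockDial actors on the lock mesh's bone sockets, passing each its index and a lock reference.
; Interacting blends to the lock camera, freezes movement, blocks inventory and shows dial arrows, with clicks routed through WidgetInteraction.
; CheckEveryTurn compares dials to LockCombination, then plays the open animation and restores player control.
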(event `Key|LeftMouseButton`
  (params (Key :type "Key Structure"))
  (bind _widgetinteraction (`self.WidgetInteraction`))
  ; Dial Interaction
  (:`Pressed`
    (`WidgetInteractionComponent.PressPointerKey` _widgetinteraction Key)
    (`WidgetInteractionComponent.ReleasePointerKey` _widgetinteraction Key)))

(event `self.ReceiveBeginPlay`
  ; Initializing Dials
  (bind _ashg_player_controller (cast `/Game/GameBP/HG_PlayerController` (`GameplayStatics.GetPlayerController` 0)))
  (set `self.PlayerControllerRef` _ashg_player_controller)
  (for _index (range 4)
    (bind _returnvalue (`|SpawnActorFromClass` "/Game/Blueprints/Actors/Lock/BP_LockDial.BP_LockDial_C" (`KismetMathLibrary.MakeTransform` (0.0 0.0 0.0)) "AlwaysSpawn" "MultiplyWithRoot" null _index self null))
    (`KismetArrayLibrary.Array_Add` (`self.Dials`) _returnvalue)
    (`self.K2_AttachToComponent` _returnvalue (`self.Lock`) (select `int` _index :`0` "DialBone1Socket" :`1` "DialBone2Socket" :`2` "DialBone3Socket" :`3` "DialBone4Socket" :!type "Name") "SnapToTarget" "KeepWorld" "KeepWorld" true)))

(event `CheckEveryTurn`
  ; Check Every Turn
  (bind _success_ (`self.CheckCode`))
  (if _success_
    (`SkeletalMeshComponent.PlayAnimation` (`self.Lock`) "/Game/Props/Animations/Lock/7_6_LockOpen.7_6_LockOpen" false)
    (`KismetSystemLibrary.Delay` 2.0)
    (`self.ExitLockVIew`)
    (`KismetSystemLibrary.Delay` 1.0)
    (`self.K2_DestroyActor`)
    (for _array_element (`self.Dials`)
      (`self.K2_DestroyActor` _array_element))))

(event `/Game/Blueprints/Interfaces/BPI_Intraction.Interact`
  (bind _returnvalue (`GameplayStatics.GetPlayerController` 0))
  ; Enter Lock View
  (`PlayerController.SetViewTargetWithBlend` (`GameplayStatics.GetPlayerController` 0) (`ActorComponent.GetOwner` (`self.Camera`)) 1.0 "VTBlend_Linear" 0.0 false)
  (`CharacterMovementComponent.DisableMovement` (`Character.CharacterMovement` (`GameplayStatics.GetPlayerCharacter` 0)))
  (`Controller.SetIgnoreLookInput` (`GameplayStatics.GetPlayerController` 0) false)
  (set `/Game/GameBP/HG_PlayerController.CanOpenInventory` false (`self.PlayerControllerRef`))
  (`KismetSystemLibrary.Delay` 1.0)
  (`self.EnableInput` _returnvalue)
  (set `PlayerController.bShowMouseCursor` true _returnvalue)
  (for _array_element (`self.Dials`)
    (`SceneComponent.SetVisibility` (`/Game/Blueprints/Actors/Lock/BP_LockDial.UpArrow` _array_element) true false)
    (`SceneComponent.SetVisibility` (`/Game/Blueprints/Actors/Lock/BP_LockDial.DownArrow` _array_element) true false)))

(event `EnhancedInput|/Game/EnhancedInputs/Actions/IA_Return`
  (params (ActionValue :type Boolean) (ElapsedSeconds :type "Float (double-precision)") (TriggeredSeconds :type "Float (double-precision)") (InputAction :type "InputAction Object Reference" :default "/Game/EnhancedInputs/Actions/IA_Return.IA_Return"))
  ; Enter Lock View
  (:`Started`
    (`self.ExitLockVIew`)))

(event `ExitLockVIew`
  (bind _returnvalue (`GameplayStatics.GetPlayerController` 0))
  (bind _returnvalue_2 (`GameplayStatics.GetPlayerCharacter` 0))
  ; Exit Lock View
  (`PlayerController.SetViewTargetWithBlend` _returnvalue _returnvalue_2 1.0 "VTBlend_Linear" 0.0 false)
  (`self.DisableInput` _returnvalue)
  (`Controller.ResetIgnoreLookInput` _returnvalue)
  (set `/Game/GameBP/HG_PlayerController.CanOpenInventory` true (`self.PlayerControllerRef`))
  (`CharacterMovementComponent.SetMovementMode` (`Character.CharacterMovement` _returnvalue_2) "MOVE_Walking" 0)
  (set `PlayerController.bShowMouseCursor` false (`GameplayStatics.GetPlayerController` 0))
  (for _array_element (`self.Dials`)
    (`SceneComponent.SetVisibility` (`/Game/Blueprints/Actors/Lock/BP_LockDial.UpArrow` _array_element) false false)
    (`SceneComponent.SetVisibility` (`/Game/Blueprints/Actors/Lock/BP_LockDial.DownArrow` _array_element) false false)))

(fn `CheckCode`
  (returns (`Success?` :type Boolean))
  (locals (LocalSuccess :type Boolean))
  (for (_array_element _array_index) (`self.Dials`)
    (if (== (`/Game/Blueprints/Actors/Lock/BP_LockDial.CorrectNumber` _array_element) (`|GetArrayItem` (`self.LockCombination`) _array_index))
      (set `local.LocalSuccess` true)
      (else
        (set `local.LocalSuccess` false)
        (break))))
  (return (`local.LocalSuccess`)))

(fn `UserConstructionScript`
  (`BoxComponent.SetBoxExtent` (`self.Box`) (`self.BoxExtent`) true)
  (`SceneComponent.K2_SetRelativeLocation` (`self.Box`) (`self.BoxPosition`) false false))