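; A single ten-digit dial for a combination lock, randomized at BeginPlay and turned through up and down arrow widgets that receive a reference to it.
; One timeline, played forward or in reverse, animates each 36-degree step, with CanRotate blocking input mid-turn.
; When a turn finishes, it wraps the stored rotation, converts it to the dial's corrected digit and tells the parent lock to check the combination.
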(event `self.ReceiveBeginPlay`
  ; Initialize Widget
  (bind _asuwb_arrow (cast `/Game/UMG/Lock/UWB_Arrow` (`WidgetComponent.GetUserWidgetObject` (`self.UpArrow`))))
  (`/Game/UMG/Lock/UWB_Arrow.Initialize` _asuwb_arrow self true)
  (bind _asuwb_arrow_2 (cast `/Game/UMG/Lock/UWB_Arrow` (`WidgetComponent.GetUserWidgetObject` (`self.DownArrow`))))
  (`/Game/UMG/Lock/UWB_Arrow.Initialize` _asuwb_arrow_2 self false)
  (`self.SetRandomNumber`))

(event `FixNumber`
  ; Fixes the number to corresponding number on dial
  (set `self.CorrectNumber` (mod (- 15 (`self.Number`)) 10)))

(event `FindNumber`
  ; Finds number based on the rotation of dial
  (set `self.Number` (`KismetMathLibrary.Abs_Int` (`KismetMathLibrary.FTrunc` (/ (`self.DialRotation`) 36.0))))
  (`self.FixNumber`))

(event `RotateDial`
  (bind _dialrotation (`self.DialRotation`))
  ; Rotates the dial
  (if (`self.CanRotate`)
    (set `self.CanRotate` false)
    (bind (_direction _alpha) (`Timeline|RotateDialTL` :!via `PlayFromStart` :!label _label)
      (:`Update`
        (bind _returnvalue (- (`self.DialRotation`) (select `ETimelineDirection` _direction :`Forward` (`KismetMathLibrary.Lerp` 0.0 36.0 _alpha) :`Backward` (`KismetMathLibrary.Lerp` -36.0 0.0 _alpha))))
        (`SceneComponent.K2_SetRelativeRotation` (`self.Dial`) (`KismetMathLibrary.MakeRotator` _returnvalue) false false))
      (:`Finished`
        (set `self.DialRotation` _returnvalue)
        (if (<= _dialrotation 0.0)
          (set `self.DialRotation` 360.0)
          (`SceneComponent.K2_SetRelativeRotation` :`self` (`self.Dial`))
          (elif (>= _dialrotation 360.0)
            (bind _output_get (set `self.DialRotation` (`KismetMathLibrary.MapRangeClamped` (`self.DialRotation`) 0.0 -360.0 360.0)))
            (`SceneComponent.K2_SetRelativeRotation` (`self.Dial`) (`KismetMathLibrary.MakeRotator` _output_get) false false)))
        (`self.FindNumber`)
        (`/Game/Blueprints/Actors/Lock/BP_Lock.CheckEveryTurn` (`self.BP_LockRef`))
        (set `self.CanRotate` true)))))

(event `RotateDialBackwards`
  ; Rotates the dial
  (if (`self.CanRotate`)
    (set `self.CanRotate` false)
    (goto _label :!via `ReverseFromEnd`)))

(fn `SetRandomNumber`
  (bind _output_get (set `self.LocalRotation` (`KismetMathLibrary.Conv_IntToDouble` (* (`KismetMathLibrary.RandomIntegerInRange` 0 9) 36))))
  (`SceneComponent.K2_SetRelativeRotation` (`self.Dial`) (`KismetMathLibrary.MakeRotator` _output_get) false false)
  (set `self.DialRotation` (`self.LocalRotation`))
  (`self.FindNumber`))

(fn `UserConstructionScript`)