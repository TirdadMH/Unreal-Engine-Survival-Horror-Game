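; Base note pickup actor with editable front and back text that opens an examination widget when the player presses IA_Action.
; Overlapping the sphere starts a per-tick line trace to the player camera, showing a camera-facing prompt above the paper while sight is unblocked.
; Within pickup distance the prompt toggles and input is enabled.
; The examination widget receives the note and the level's BP_NoteExamineAction reference.
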(event `self.ReceiveBeginPlay`
  (bind _returnvalue (`GameplayStatics.GetActorOfClass` "/Game/Blueprints/Actors/Notes/BP_NoteExamineAction.BP_NoteExamineAction_C"))
  (set `self.BP_NoteExamineActionRef` _returnvalue))

(event `self.OverlapsSphere.OnComponentBeginOverlap`
  (params (OverlappedComponent :type "PrimitiveComponent Object Reference") (OtherActor :type "Actor Object Reference") (OtherComp :type "PrimitiveComponent Object Reference") (OtherBodyIndex :type Integer) (bFromSweep :type Boolean) (SweepResult :type "HitResult Structure (by ref)"))
  (bind _asl1_character (cast `/Game/GameBP/LevelOne/L1_Character` OtherActor))
  (set `self.PlayerRef` _asl1_character)
  (`SceneComponent.SetVisibility` (`self.Widget`) true false)
  (set `self.UpdateActor` true))

(event `self.OverlapsSphere.OnComponentEndOverlap`
  (params (OverlappedComponent :type "PrimitiveComponent Object Reference") (OtherActor :type "Actor Object Reference") (OtherComp :type "PrimitiveComponent Object Reference") (OtherBodyIndex :type Integer))
  (cast `/Game/GameBP/LevelOne/L1_Character` OtherActor)
  (`SceneComponent.SetVisibility` (`self.Widget`) false false)
  (set `self.UpdateActor` false)
  (`self.DisableInput` (`GameplayStatics.GetPlayerController` 0)))

(event `EnhancedInput|/Game/EnhancedInputs/Actions/IA_Action`
  (params (ActionValue :type Boolean) (ElapsedSeconds :type "Float (double-precision)") (TriggeredSeconds :type "Float (double-precision)") (InputAction :type "InputAction Object Reference" :default "/Game/EnhancedInputs/Actions/IA_Action.IA_Action"))
  (:`Started`
    (bind _returnvalue (`|CreateWidget` "/Game/UMG/Inventory/UWB_NoteExamination.UWB_NoteExamination_C" null (`self.BP_NoteExamineActionRef`)))
    (`/Game/UMG/Inventory/UWB_NoteExamination.UpdateWidget` _returnvalue self)
    (`UserWidget.AddToViewport` _returnvalue 0)))

(event `self.ReceiveTick`
  (params (DeltaSeconds :type "Float (single-precision)"))
  (bind _returnvalue (`GameplayStatics.GetPlayerController` 0))
  (bind (_returnvalue_x _returnvalue_y _returnvalue_z) (`KismetMathLibrary.BreakVector` (`SceneComponent.K2_GetComponentLocation` (`self.PaperMesh`))))
  (`SceneComponent.K2_SetWorldLocation` (`self.Widget`) (`KismetMathLibrary.MakeVector` _returnvalue_x _returnvalue_y (+ _returnvalue_z (`self.WIdgetDistanceAboveMesh`))) false false)
  (if (`self.UpdateActor`)
    (bind (_outhit _returnvalue_2) (`KismetSystemLibrary.LineTraceSingle` (`self.K2_GetActorLocation`) (`SceneComponent.K2_GetComponentLocation` (`/Game/GameBP/LevelOne/L1_Character.Camera` (`self.PlayerRef`))) "TraceTypeQuery1"))
    (if (not _returnvalue_2)
      (`SceneComponent.SetVisibility` (`self.Widget`) true false)
      (`SceneComponent.K2_SetWorldRotation` (`self.Widget`) (`KismetMathLibrary.FindLookAtRotation` (`SceneComponent.K2_GetComponentLocation` (`self.Widget`)) (`SceneComponent.K2_GetComponentLocation` (`/Game/GameBP/LevelOne/L1_Character.Camera` (`self.PlayerRef`)))) false false)
      (bind (_bblockinghit _binitialoverlap _time _distance _location _impactpoint _normal _impactnormal _physmat _hitactor _hitcomponent _hitbonename _bonename _hititem _elementindex _faceindex _tracestart _traceend) (`GameplayStatics.BreakHitResult` _outhit))
      (bind _returnvalue_3 (<= (`KismetMathLibrary.VSize` (- _tracestart _traceend)) (`self.PickupDistance`)))
      (`/Game/UMG/Inventory/UWB_PickupPrompt.TogglePrompt` (cast `/Game/UMG/Inventory/UWB_PickupPrompt` (`WidgetComponent.GetUserWidgetObject` (`self.Widget`)) :!pure true) _returnvalue_3)
      (if _returnvalue_3
        (`self.EnableInput` _returnvalue)
        (else
          (`self.DisableInput` _returnvalue)))
      (else
        (`SceneComponent.SetVisibility` (`self.Widget`) false false)
        (`self.DisableInput` (`GameplayStatics.GetPlayerController` 0))))))

(fn `UserConstructionScript`
  (`TextRenderComponent.K2_SetText` (`self.NoteText`) (`self.NoteText(Text)`))
  (`TextRenderComponent.K2_SetText` (`self.BackNoteText`) (`self.BackNoteText(Text)`)))