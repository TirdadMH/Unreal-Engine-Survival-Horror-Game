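; Player flashlight component that toggles the player's light and manages its battery charge.
; Initialize caches the player's Flashlight and sets the starting charge; toggling on requires charge above minimum and starts a looping depletion timer.
; Depleting and adding charge both clamp the level and update IES brightness scale, which fades only below a charge of 20.
; Reaching minimum charge turns the light off and clears the timer.
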(fn `AddBatteryLife`
  (params (Amount :type "Float (double-precision)"))
  (set `self.CurrentBatteryLevel` (`KismetMathLibrary.FClamp` (+ Amount (`self.CurrentBatteryLevel`)) (`self.MinBatteryLevel`) (`self.MaxBatteryLevel`)))
  (`self.SetIntencity`))

(fn `DepleteBatteryLife`
  (bind _output_get (set `self.CurrentBatteryLevel` (`KismetMathLibrary.FClamp` (- (`self.CurrentBatteryLevel`) (`self.DelpletionAmount`)) (`self.MinBatteryLevel`) (`self.MaxBatteryLevel`))))
  (`self.SetIntencity`)
  (if (<= _output_get (`self.MinBatteryLevel`))
    (`SceneComponent.SetVisibility` (`self.FlashlightLight`) false false)
    (`KismetSystemLibrary.K2_ClearTimer` null "DepleteBatteryLife")))

(fn `Initialize`
  (params (Player :type "/Game/GameBP/LevelOne/L1_Character Object Reference"))
  (bind _output_get (set `self.PlayerRef` Player))
  (set `self.FlashlightLight` (`/Game/GameBP/LevelOne/L1_Character.Flashlight` _output_get))
  (set `self.CurrentBatteryLevel` (`self.InitializedBatteryLevel`)))

(fn `SetIntencity`
  ; Starts fading at 20%, because it's clamped
  (`LightComponent.SetIESBrightnessScale` (`self.FlashlightLight`) (`KismetMathLibrary.MapRangeClamped` (`self.CurrentBatteryLevel`) (`self.MinBatteryLevel`) 20.0 0.0 1.0)))

(fn `ToggleFlashlight`
  (bind _flashlightlight (`self.FlashlightLight`))
  ;[1 1 1] Toggle
  (if (`SceneComponent.bVisible` _flashlightlight)
    (`SceneComponent.SetVisibility` _flashlightlight false false)
    (`KismetSystemLibrary.K2_ClearTimer` null "DepleteBatteryLife")
    (elif (> (`self.CurrentBatteryLevel`) (`self.MinBatteryLevel`))
      (`self.SetIntencity`)
      (`SceneComponent.SetVisibility` _flashlightlight true false)
      (`KismetSystemLibrary.K2_SetTimer` null "DepleteBatteryLife" (`self.DepletionSpeed`) true))))