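; Health component that tracks a clamped health value and drives a blood screen effect.
; AddHealth and RemoveHealth adjust CurrentHealth within its minimum and maximum, then refresh the effect, which is also initialized on BeginPlay.
; UpdateBloodScreen maps health below a StartAtNumber fraction of the health range to the Radius scalar in the MPC_BloodScreen material parameter collection.
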(event `self.ReceiveBeginPlay`
  (`self.UpdateBloodScreen`))

(fn `AddHealth`
  (params (Amount :type "Float (double-precision)"))
  (set `self.CurrentHealth` (`KismetMathLibrary.FClamp` (+ Amount (`self.CurrentHealth`)) (`self.MinHealth`) (`self.MaxHealth`)))
  (`self.UpdateBloodScreen`))

(fn `RemoveHealth`
  (params (Amount :type "Float (double-precision)"))
  (set `self.CurrentHealth` (`KismetMathLibrary.FClamp` (- (`self.CurrentHealth`) Amount) (`self.MinHealth`) (`self.MaxHealth`)))
  (`self.UpdateBloodScreen`))

(fn `UpdateBloodScreen`
  (locals (StartAtNumber :type "Float (double-precision)" :default 0.7))
  (`KismetMaterialLibrary.SetScalarParameterValue` "/Game/Materials/UI/MPC_BloodScreen.MPC_BloodScreen" "Radius" (`KismetMathLibrary.MapRangeClamped` (`self.CurrentHealth`) (`self.MinHealth`) (* (- (`self.MaxHealth`) (`self.MinHealth`)) (`local.StartAtNumber`)) 0.5 1.0)))