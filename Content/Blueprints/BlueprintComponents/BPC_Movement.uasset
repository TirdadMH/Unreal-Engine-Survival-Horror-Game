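; Movement component that gives a player character stamina-limited sprinting and crouching.
; Initialize stores the character reference; sprint and crouch events then set its max walk speed, with crouching also resizing the capsule through L1_Character.
; Looping named timers drain stamina while sprinting, stopping at the minimum, and refill it after a retriggerable delay following StopSprint.
; Starting a sprint ends crouch and cancels regeneration, while crouching cancels the drain timer.
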(event `StartSprint`
  ;[1 1 1] Sprinting
  ;;[1 1 1] Start Sprinting
  (if (`self.IsCrouching`)
    (`self.EndCrouch`))
  (`KismetSystemLibrary.K2_ClearTimer` null "RegenerateStamina")
  (if (> (`self.CurrentStamina`) (`self.MinStamina`))
    (set `CharacterMovementComponent.MaxWalkSpeed` (`self.SprintSpeed`) (`Character.CharacterMovement` (`self.PlayerRef`)))
    (`KismetSystemLibrary.K2_SetTimer` null "SprintTimer" 0.1 true)))

(event `SprintTimer`
  ;[1 1 1] Sprinting
  ;;[1 1 1] Sprint Timer
  (bind _output_get (set `self.CurrentStamina` (`KismetMathLibrary.FClamp` (- (`self.CurrentStamina`) 1.0) (`self.MinStamina`) (`self.MaxStamina`))))
  (if (<= _output_get (`self.MinStamina`))
    (`self.StopSprint`)))

(event `StopSprint`
  ;[1 1 1] Sprinting
  ;;[1 1 1] Stop Sprinting
  (if (not (`self.IsCrouching`))
    (`KismetSystemLibrary.K2_ClearTimer` null "SprintTimer")
    (set `CharacterMovementComponent.MaxWalkSpeed` (`self.WalkSpeed`) (`Character.CharacterMovement` (`self.PlayerRef`)))
    (`KismetSystemLibrary.RetriggerableDelay` 5.0)
    (if (not (`KismetSystemLibrary.K2_IsTimerActive` null "SprintTimer"))
      (`KismetSystemLibrary.K2_SetTimer` null "RegenerateStamina" 0.03 true))))

(event `RegenerateStamina`
  ;[1 1 1] Sprinting
  ;;[1 1 1] Regenerate Stamina
  (bind _output_get (set `self.CurrentStamina` (`KismetMathLibrary.FClamp` (+ (`self.CurrentStamina`) 1.0) (`self.MinStamina`) (`self.MaxStamina`))))
  (if (>= _output_get (`self.MaxStamina`))
    (`KismetSystemLibrary.K2_ClearTimer` null "RegenerateStamina")))

(event `StartCrouch`
  ;[1 1 1] Crouch
  (`KismetSystemLibrary.K2_ClearTimer` null "SprintTimer")
  (set `CharacterMovementComponent.MaxWalkSpeed` (`self.CrouchSpeed`) (`Character.CharacterMovement` (`self.PlayerRef`)))
  (`/Game/GameBP/LevelOne/L1_Character.ShortenPlayerCapsule` (cast `/Game/GameBP/LevelOne/L1_Character` (`self.PlayerRef`) :!pure true))
  (set `self.IsCrouching` true))

(event `EndCrouch`
  ;[1 1 1] Crouch
  (set `CharacterMovementComponent.MaxWalkSpeed` (`self.WalkSpeed`) (`Character.CharacterMovement` (`self.PlayerRef`)))
  (`/Game/GameBP/LevelOne/L1_Character.LenghtenPlayerCapsule` (cast `/Game/GameBP/LevelOne/L1_Character` (`self.PlayerRef`) :!pure true))
  (set `self.IsCrouching` false))

(fn `Initialize`
  (params (Character :type "Character Object Reference"))
  (bind _output_get (set `self.PlayerRef` Character))
  (set `CharacterMovementComponent.MaxWalkSpeed` (`self.WalkSpeed`) (`Character.CharacterMovement` _output_get)))